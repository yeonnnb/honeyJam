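; NPC actor that walks a character along a spline to board a bus, then hands it off to a seated version.
; After a one-second wait, Tick advances the character by Speed; at the spline's end the actor destroys itself.
; Up to eight random tries seek a free GameInstance seat, spawning BP_Spline_Sit_Orange_W there and flagging it TheMan when the total count matches.
; Capsule overlap with a "trigger"-tagged actor briefly shows a profile widget.
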(event OnComponentBeginOverlap(Capsule)
  (params (OverlappedComponent :type Primitive%20Component%20Object%20Reference) (OtherActor :type Actor%20Object%20Reference) (OtherComp :type Primitive%20Component%20Object%20Reference) (OtherBodyIndex :type Integer) (bFromSweep :type Boolean) (SweepResult :type Hit%20Result%20Structure%20%28by%20ref%29))
  ;[1 1 1] 버스에 탑승시 프로필 보이기
  (Variables|Default|SetOther%20Actor OtherActor)
  (if (Actor|ActorHasTag OtherActor "trigger")
    (bind _returnvalue (UserInterface|CreateWidget "/Game/UI/ProfileWidget.ProfileWidget_C"))
    (UserInterface|Viewport|AddtoViewport _returnvalue 0)
    (Utilities|FlowControl|Delay 1.2)
    (Widget|RemovefromParent _returnvalue)))

(event EventTick
  (params (DeltaSeconds :type Float%20%28single-precision%29))
  (bind _returnvalue (Game|GetGameInstance))
  (bind _asgi (Utilities|Casting|CastToGI _returnvalue))
  (bind _npc_sit (Variables|/Game/GI.GI_C|GetNPC_Sit _asgi))
  (bind _npc_totalcount (Variables|/Game/GI.GI_C|GetNPC_TotalCount _asgi))
  (bind _output_get (Variables|Default|SetTime (+ DeltaSeconds (Variables|Default|GetTime))))
  (if (> _output_get 1.0)
    (Variables|Default|SetDistance%20along%20Spline (+ (* DeltaSeconds (Variables|Default|GetSpeed)) (Variables|Default|GetDistance%20along%20Spline)))
    (Transformation|SetRelativeTransform (Variables|Default|GetCharacter) (Math|Transform|MakeTransform (Math|Vector|MakeVector (.x (.location (Spline|GetTransformatDistanceAlongSpline (Variables|Default|GetSpline) (Variables|Default|GetDistance%20along%20Spline) "Local" false))) (.y (.location (Spline|GetTransformatDistanceAlongSpline (Variables|Default|GetSpline) (Variables|Default|GetDistance%20along%20Spline) "Local" false))) (+ (.z (.location (Spline|GetTransformatDistanceAlongSpline (Variables|Default|GetSpline) (Variables|Default|GetDistance%20along%20Spline) "Local" false))) -9e+01)) (Math|Rotator|MakeRotator (.roll (.rotation (Spline|GetTransformatDistanceAlongSpline (Variables|Default|GetSpline) (Variables|Default|GetDistance%20along%20Spline) "Local" false))) (.pitch (.rotation (Spline|GetTransformatDistanceAlongSpline (Variables|Default|GetSpline) (Variables|Default|GetDistance%20along%20Spline) "Local" false))) (+ (.yaw (.rotation (Spline|GetTransformatDistanceAlongSpline (Variables|Default|GetSpline) (Variables|Default|GetDistance%20along%20Spline) "Local" false))) -9e+01)) (Variables|/Script/Engine.SceneComponent|GetRelativeScale3D (Variables|Default|GetCharacter))) false false)
    ;[1 1 1] spline길이와 캐릭터의 도착 지점이 같으면 버스자리에 앉기
    (if (>= (Variables|Default|GetDistance%20along%20Spline) (Spline|GetSplineLength (Variables|Default|GetSpline)))
      (Actor|DestroyActor)
      (Utilities|FlowControl|ForLoopwithBreak 0 7 :!label _label
        (:LoopBody
          (Variables|Default|SetSit_Num (Math|Random|RandomInteger 8))
          (if (not (Utilities|Array|Get(acopy) _npc_sit (Variables|Default|GetSit_Num)))
            (Utilities|Array|SetArrayElem _npc_sit (Variables|Default|GetSit_Num) true)
            (Math|Integer|IncrementInt (Variables|/Game/GI.GI_C|GetNPC_Count _asgi)
              (:%20%20
                (bind _returnvalue_2 (Game|SpawnActorfromClass "/Game/NPC/BP_Spline_Sit_Orange_W.BP_Spline_Sit_Orange_W_C" (Math|Transform|MakeTransform (Utilities|Array|Get(acopy) (Variables|/Game/GI.GI_C|GetNPC_Position _asgi) (Variables|Default|GetSit_Num)) "0, 0, 0" "1.000000,1.000000,1.000000") "Undefined" 0 (Variables|Default|GetSit_Num) 0))
                (Math|Integer|IncrementInt _npc_totalcount
                  (:%20%20
                    (if (== (Variables|/Game/GI.GI_C|GetTheMan _asgi) _npc_totalcount)
                      (Variables|/Game/NPC/BP_Spline_Sit_Orange_W.BP_Spline_Sit_Orange_W_C|SetTheMan _returnvalue_2 true)
                      (goto _label Break)
                      (else
                        (goto _label Break)))))))))))))

(fn ConstructionScript)