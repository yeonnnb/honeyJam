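; Seated Orange NPC that animates with the game state, can drop honey, and may leave when a door opens.
; Tick picks jam, sit or random animation classes from Jam and the GameInstance's IsStop.
; While not stopped, rare rolls fire a DoOnce honey spawn varying by TheMan, briefly setting Jam.
; Each OpenDoor cycle after the first gives a one-in-four chance to update its NPCSit slot and destroy itself.
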(event EventTick
  (params (DeltaSeconds :type Float%20%28single-precision%29))
  (bind _returnvalue (Transformation|GetActorLocation))
  (bind _returnvalue_2 (Transformation|GetActorLocation))
  (bind _returnvalue_3 (Game|GetGameInstance))
  (bind _asgi (Utilities|Casting|CastToGI _returnvalue_3))
  (bind _opendoor (Variables|/Game/GI.GI_C|GetOpenDoor _asgi))
  (Utilities|FlowControl|Sequence
    (:then_0
      (if (Variables|Default|GetJam)
        (Class|SkeletalMeshComponent|SetAnimClass (Variables|Default|GetCharacter) "/Game/NPC/Orange_M_jam.Orange_M_jam_C")
        (elif (Variables|/Game/GI.GI_C|GetIsStop _asgi)
          (Class|SkeletalMeshComponent|SetAnimClass (Variables|Default|GetCharacter) "/Game/NPC/Orange_sit.Orange_sit_C")
          (else
            (Class|SkeletalMeshComponent|SetAnimClass (Variables|Default|GetCharacter) "/Game/NPC/Orange_random.Orange_random_C")
            (if (and (Variables|Default|GetTheMan) (== (Math|Random|RandomInteger 1000) 1))
              (Utilities|FlowControl|DoOnce false
                (:Completed
                  (Game|SpawnActorfromClass "/Game/Jam/honey/BP_Honey.BP_Honey_C" (Math|Transform|MakeTransform (Math|Vector|MakeVector (+ (Math|Random|RandomFloatinRange -15.0 15.0) (.x _returnvalue)) (+ (.y _returnvalue) (Math|Random|RandomFloatinRange -1e+01 1e+01)) (- (.z _returnvalue) 5e+01)) "0, 0, 0" "1.000000,1.000000,1.000000") "Undefined" 0 0)
                  (Variables|Default|SetJam true :!label _label)
                  (Utilities|FlowControl|Delay 1.0)
                  (Variables|Default|SetJam false)))
              (elif (and (not (Variables|Default|GetTheMan)) (== (Math|Random|RandomInteger 1000) 1))
                (Utilities|FlowControl|DoOnce false
                  (:Completed
                    (if (== (Math|Random|RandomInteger 2) 1)
                      (Game|SpawnActorfromClass "/Game/Jam/honey/BP_Honey_2.BP_Honey_2_C" (Math|Transform|MakeTransform (Math|Vector|MakeVector (+ (Math|Random|RandomFloatinRange -15.0 15.0) (.x _returnvalue_2)) (+ (.y _returnvalue_2) (Math|Random|RandomFloatinRange -1e+01 1e+01)) (- (.z _returnvalue_2) 5e+01)) "0, 0, 0" "1.000000,1.000000,1.000000") "Undefined" 0 0)
                      (goto _label))))))))))
    (:then_1
      (if _opendoor
        (Utilities|FlowControl|DoOnce false :!label _label_2
          (:Completed
            (if (Variables|Default|GetStayOnce)
              (if (== (Math|Random|RandomInteger 4) 1)
                (Utilities|Array|SetArrayElem (Variables|/Game/GI.GI_C|GetNPC_Sit _asgi) (Variables|Default|GetSitNum) false)
                (Actor|DestroyActor))
              (else
                (Variables|Default|SetStayOnce true)))))))
    (:then_2
      (if (not _opendoor)
        (goto _label_2 Reset)))))

(fn ConstructionScript)